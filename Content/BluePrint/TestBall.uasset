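; TestBall is a test actor that follows the player pawn, with a Sphere component placed on an elliptical offset around it.
; Each Tick snaps the actor to player 0's pawn, then sets the sphere's relative location from cosine and sine of Time, scaled by X and Y.
; Time resets when Time plus the Speed-scaled delta reaches 360, but otherwise is written back unchanged, so the angle never advances as written.
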(event `self.ReceiveTick`
  (params (DeltaSeconds :type "Float (single-precision)"))
  (bind _time (`self.time`))
  (bind _time_2 (`self.time`))
  ;[1 1 1] Comment
  (`self.K2_SetActorLocation` (`self.K2_GetActorLocation` (`GameplayStatics.GetPlayerPawn` 0)))
  (`SceneComponent.K2_SetRelativeLocation` (`self.Sphere`) (`KismetMathLibrary.MakeVector` (* (`KismetMathLibrary.DegCos` _time) (`self.x`)) (* (`KismetMathLibrary.DegSin` _time) (`self.y`))) false false)
  (if (>= (+ _time_2 (* (`GameplayStatics.GetWorldDeltaSeconds`) (`self.speed`))) 360.0)
    (set `self.time` 0.0)
    (else
      (set `self.time` _time_2))))

(fn `UserConstructionScript`)